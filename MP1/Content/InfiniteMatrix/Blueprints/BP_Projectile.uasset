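; BP_Projectile is a projectile that scores points for the player by destroying enemies it overlaps.
; On overlap it ignores BP_Player; a BP_Enemy hit adds to the first player pawn's Score, then destroys that enemy after a short delay.
; Overlapping any other actor destroys the projectile after a short delay, while enemy hits leave it alive.
; No movement logic appears in its graphs.
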(event Collision|EventActorBeginOverlap
  (params (OtherActor :type Actor%20Object%20Reference))
  (Utilities|Casting|CastToBP_Player OtherActor
    (:CastFailed
      (bind _asbp_enemy (Utilities|Casting|CastToBP_Enemy OtherActor)
        (:then
          (bind _asbp_player (Utilities|Casting|CastToBP_Player (Game|Player|GetPlayerPawn 0)))
          (Variables|/Game/InfiniteMatrix/Blueprints/BP_Player.BP_Player_C|SetScore _asbp_player (+ (Variables|/Game/InfiniteMatrix/Blueprints/BP_Player.BP_Player_C|GetScore _asbp_player) 2))
          (Utilities|FlowControl|Delay 0.154)
          (Actor|DestroyActor _asbp_enemy))
        (:CastFailed
          (Utilities|FlowControl|Delay 0.2)
          (Actor|DestroyActor))))))

(event EventTick
  (params (DeltaSeconds :type Float%20%28single-precision%29)))

(fn ConstructionScript)